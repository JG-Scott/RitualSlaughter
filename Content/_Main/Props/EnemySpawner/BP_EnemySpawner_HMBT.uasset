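; Enemy spawner that periodically spawns a random HMBT Scout, BigBoy or Cultist group at nearby navigable points while enabled and below its enemy cap.
; Tick runs the countdown; cultist groups have random size, can overshoot the cap, and assign the first member as leader through the others' AI controllers.
; Spawned enemies hold a spawner reference; EnemyDeath decrements the count and calls SpawnerCleared on BP_FirstPersonGameMode at zero.
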(event Custom|SpawnRandomEnemy
  (switch int (Math|Random|RandomIntegerinRange 0 2)
    (:0
      (CallFunction|SpawnScout))
    (:1
      (CallFunction|SpawnBigBoy))
    (:2
      (CallFunction|SpawnCultist))))

(event Custom|SpawnCultist
  (CallFunction|SpawnHMBTCultists))

(event Custom|SpawnScout
  (bind _randomlocation (Utilities|GetRandomLocation))
  (bind _returnvalue (Game|SpawnActorfromClass "/Game/_Main/Enemies/Rough/HomeMadeBehaviorTreeEnemies/BP_HMBT_Scout.BP_HMBT_Scout_C" (Math|Transform|MakeTransform _randomlocation "0, 0, 0" "1.000000,1.000000,1.000000") "AdjustIfPossibleButAlwaysSpawn" "MultiplyWithRoot" 0 0))
  (Variables|/Game/_Main/Enemies/Rough/BP_EnemyBase.BP_EnemyBase_C|SetSpawner _returnvalue self)
  (Math|Integer|IncrementInt (Variables|Default|GetCurrentEnemyAmount)))

(event Custom|SpawnBigBoy
  (bind _randomlocation (Utilities|GetRandomLocation))
  (bind _returnvalue (Game|SpawnActorfromClass "/Game/_Main/Enemies/Rough/HomeMadeBehaviorTreeEnemies/BP_HMBT_BigBoy.BP_HMBT_BigBoy_C" (Math|Transform|MakeTransform _randomlocation "0, 0, 0" "1.000000,1.000000,1.000000") "AdjustIfPossibleButAlwaysSpawn" "MultiplyWithRoot" 0 0))
  (Variables|/Game/_Main/Enemies/Rough/BP_EnemyBase.BP_EnemyBase_C|SetSpawner _returnvalue self)
  (Math|Integer|IncrementInt (Variables|Default|GetCurrentEnemyAmount)))

(event Custom|EnemyDeath
  (bind _result (Math|Integer|DecrementInt (Variables|Default|GetCurrentEnemyAmount))
    (:%20%20
      (if (<= _result 0)
        (bind _asbp_first_person_game_mode (Utilities|Casting|CastToBP_FirstPersonGameMode (Game|GetGameMode)))
        (Default|SpawnerCleared _asbp_first_person_game_mode)))))

(event EventBeginPlay
  (Variables|Default|SetSpawnTimerOriginal (Variables|Default|GetSpawnTimer)))

(event Collision|EventActorBeginOverlap
  (params (OtherActor :type Actor%20Object%20Reference)))

(event EventTick
  (params (DeltaSeconds :type Float%20%28single-precision%29))
  (if (Variables|Default|GetCanSpawnEnemies)
    (if (< (Variables|Default|GetCurrentEnemyAmount) (Variables|Default|GetMaximumEnemyAmount))
      (bind _output_get (Variables|Default|SetSpawnTimer (- (Variables|Default|GetSpawnTimer) DeltaSeconds)))
      (if (<= _output_get 0.0)
        (Variables|Default|SetSpawnTimer (Variables|Default|GetSpawnTimerOriginal))
        (CallFunction|SpawnRandomEnemy)))))

(fn ConstructionScript)

(fn SpawnHMBTCultists
  (for _index (range 0 (Math|Random|RandomIntegerinRange (Variables|Default|GetMinimumCultistGroupAmount) (Variables|Default|GetMaximumCultistGroupAmount)))
    (if (== _index 0)
      (bind _randomlocation (Utilities|GetRandomLocation))
      (bind _returnvalue (Game|SpawnActorfromClass "/Game/_Main/Enemies/Rough/HomeMadeBehaviorTreeEnemies/BP_HMBT_Cultist.BP_HMBT_Cultist_C" (Math|Transform|MakeTransform _randomlocation "0, 0, 0" "1.000000,1.000000,1.000000") "AdjustIfPossibleButAlwaysSpawn" "MultiplyWithRoot" 0 0))
      (Variables|/Game/_Main/Enemies/Rough/BP_EnemyBase.BP_EnemyBase_C|SetSpawner _returnvalue self)
      (LocalVariables|SetLeader _returnvalue)
      (Math|Integer|IncrementInt (Variables|Default|GetCurrentEnemyAmount))
      (else
        (bind _randomlocation_2 (Utilities|GetRandomLocation))
        (bind _returnvalue_2 (Game|SpawnActorfromClass "/Game/_Main/Enemies/Rough/HomeMadeBehaviorTreeEnemies/BP_HMBT_Cultist.BP_HMBT_Cultist_C" (Math|Transform|MakeTransform _randomlocation_2 "0, 0, 0" "1.000000,1.000000,1.000000") "AdjustIfPossibleButAlwaysSpawn" "MultiplyWithRoot" 0 0))
        (Variables|/Game/_Main/Enemies/Rough/BP_EnemyBase.BP_EnemyBase_C|SetSpawner _returnvalue_2 self)
        (bind _asaic_hmbt_cultist (Utilities|Casting|CastToAIC_HMBT_Cultist (AI|GetAIController _returnvalue_2)))
        (Default|SetLeader _asaic_hmbt_cultist (LocalVariables|GetLeader))
        (Math|Integer|IncrementInt (Variables|Default|GetCurrentEnemyAmount))))))