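; BP_HMBT_BigBoy is an enemy character for the custom "home-made" behavior tree AI that can rally nearby enemies.
; AlertSurroundings finds enemies overlapping its AlertSphere and pushes an Attack or Investigate state into their AI controllers, resetting their trees if their blackboard state differs.
; SetMovementSpeed maps standing, walking and running to max walk speed and returns it.
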(event Custom|AlertSurroundings
  (params (PlayerLocation :type Vector) (StateToSwapTo :type Enum_EnemyState%20Enum :default "NewEnumerator0") (AttackObject :type Actor%20Object%20Reference))
  (for _array_element (Collision|GetOverlappingActors (Variables|Default|GetAlertSphere) "/Game/_Main/Enemies/Rough/BP_EnemyBase.BP_EnemyBase_C" :!class /Script/Engine.PrimitiveComponent)
    (bind _asaic_hmbt_enemy_base (Utilities|Casting|CastToAIC_HMBT_Enemy_Base (AI|GetAIController _array_element)))
    (if (Utilities|Enum|NotEqual(Enum) (.state (Variables|/Game/_Main/Enemies/AI/HomeMadeBehaviorTree/AIC_HMBT_Enemy_Base.AIC_HMBT_Enemy_Base_C|GetCustomBlackBoard _asaic_hmbt_enemy_base)) StateToSwapTo)
      (switch Utilities|FlowControl|Switch|SwitchonEnum_EnemyState StateToSwapTo
        (:NewEnumerator3
          (Default|SetStateasAttacking _asaic_hmbt_enemy_base AttackObject)
          (Default|ResetBehaviorTree _asaic_hmbt_enemy_base))
        (:NewEnumerator4
          (Default|SetStateasInvestigating _asaic_hmbt_enemy_base PlayerLocation)
          (Default|ResetBehaviorTree _asaic_hmbt_enemy_base))))))

(event EventBeginPlay)

(event Collision|EventActorBeginOverlap
  (params (OtherActor :type Actor%20Object%20Reference)))

(event EventTick
  (params (DeltaSeconds :type Float%20%28single-precision%29)))

(fn ConstructionScript
  (|CallParentFunction))

(fn SetMovementSpeed
  (params (Movement%20Type :type Enum_EnemyMovementType%20Enum :default "NewEnumerator0"))
  (bind _output_get (Variables|/Script/Engine.CharacterMovementComponent|SetMaxWalkSpeed (Variables|Character|GetCharacterMovement) (Utilities|Select :Index Movement%20Type :NewEnumerator0 0.0 :NewEnumerator1 6e+02 :NewEnumerator2 9e+02)))
  (return _output_get))