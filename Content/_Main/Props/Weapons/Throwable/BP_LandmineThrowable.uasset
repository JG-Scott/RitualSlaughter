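; BP_LandmineThrowable is the thrown form of a landmine weapon, which turns into a placed landmine where it lands.
; When its solid box collision hits something, it spawns the NS_BloodExplosion1 Niagara effect and plays a ground-placement sound.
; It then spawns BP_LandminePlaced slightly above the impact point and destroys itself.
; The sphere overlap and BeginPlay events do nothing.
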(event OnComponentBeginOverlap(SphereOverlapCollision)
  (params (OverlappedComponent :type Primitive%20Component%20Object%20Reference) (OtherActor :type Actor%20Object%20Reference) (OtherComp :type Primitive%20Component%20Object%20Reference) (OtherBodyIndex :type Integer) (bFromSweep :type Boolean) (SweepResult :type Hit%20Result%20Structure%20%28by%20ref%29)))

(event OnComponentHit(BoxSolidCollision)
  (params (HitComponent :type Primitive%20Component%20Object%20Reference) (OtherActor :type Actor%20Object%20Reference) (OtherComp :type Primitive%20Component%20Object%20Reference) (NormalImpulse :type Vector :default "0, 0, 0") (Hit :type Hit%20Result%20Structure%20%28by%20ref%29))
  (bind _location (Collision|BreakHitResult Hit))
  (bind (_x _y _z) (Math|Vector|BreakVector _location))
  (Niagara|SpawnSystematLocation "/Game/_Main/ParticleEffects/ThrowableItemParticles/NS_BloodExplosion1.NS_BloodExplosion1" (Transformation|GetWorldLocation (Variables|Default|GetBoxSolidCollision)))
  (Audio|PlaySoundatLocation "/Game/_Main/Sounds/WeaponSoundEffects/LandminePlaceOnGroundSoundEffect.LandminePlaceOnGroundSoundEffect" _location "0, 0, 0" 1.0 1.0 0.0 0 0 0 0)
  (Game|SpawnActorfromClass "/Game/_Main/Props/Weapons/BP_LandminePlaced.BP_LandminePlaced_C" (Math|Transform|MakeTransform (Math|Vector|MakeVector _x _y (+ _z 5.0)) "0, 0, 0" "1.000000,1.000000,1.000000") "Undefined" "MultiplyWithRoot" 0 0)
  (Actor|DestroyActor))

(event EventBeginPlay)

(event Collision|EventActorBeginOverlap
  (params (OtherActor :type Actor%20Object%20Reference))
  (|CallParentFunction OtherActor) ; This node is disabled and will not be called.\nDrag off pins to build functionality.
)

(fn ConstructionScript
  (|CallParentFunction))