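; Shotgun weapon Blueprint that supplies the weapon's firing animation, spread hit detection and equip sound.
; GenerateRayCast loops several complex multi-line traces on the Camera channel, each ending at the Direction vector plus a random per-axis WeaponSpread offset.
; Every hit is appended to the HitResult array; damage is not applied here.
; HandleAnimation plays the fire animation on WeaponModel, and PlayEquipSound plays a 2D equip sound.
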(event EventBeginPlay
  (|CallParentFunction) ; This node is disabled and will not be called.\nDrag off pins to build functionality.
)

(event Collision|EventActorBeginOverlap
  (params (OtherActor :type Actor%20Object%20Reference))
  (|CallParentFunction OtherActor) ; This node is disabled and will not be called.\nDrag off pins to build functionality.
)

(event EventTick
  (params (DeltaSeconds :type Float%20%28single-precision%29))
  (|CallParentFunction DeltaSeconds) ; This node is disabled and will not be called.\nDrag off pins to build functionality.
)

(event EventPlayEquipSound
  (Audio|PlaySound2D "/Game/_Main/Sounds/WeaponSoundEffects/EquipWeaponitemSound.EquipWeaponitemSound" 1.0 1.0 0.0 0 0))

(event EventHandleAnimation
  (Components|Animation|PlayAnimation (Variables|Default|GetWeaponModel) "/Game/MilitaryWeapDark/Weapons/Anims/Fire_Shotgun_W.Fire_Shotgun_W" false))

(event EventGenerateRayCast
  (params (Location :type Vector :default "0, 0, 0") (Direction :type Vector :default "0, 0, 0") (IgnoreableObjects :type Array%20of%20Actor%20Object%20References))
  (bind _weaponspread (Variables|Default|GetWeaponSpread))
  (bind _returnvalue (* _weaponspread -1.0))
  (for _index (range 0 6)
    (bind _outhits (Collision|MultiLineTraceByChannel Location (+ Direction (Math|Vector|MakeVector (Math|Random|RandomFloatinRange _returnvalue _weaponspread) (Math|Random|RandomFloatinRange _returnvalue _weaponspread) (Math|Random|RandomFloatinRange _returnvalue _weaponspread))) "TraceTypeQuery2" true IgnoreableObjects "None"))
    (for _array_element _outhits
      (Utilities|Array|Add (Variables|Default|GetHitResult) _array_element))))

(fn ConstructionScript
  (|CallParentFunction))