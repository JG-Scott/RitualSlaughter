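; Rifle weapon Blueprint that supplies the rifle's firing animation and equip sound.
; HandleAnimation plays the rifle fire animation once on the WeaponModel mesh, and PlayEquipSound plays a non-spatialized 2D equip sound.
; The default BeginPlay, overlap and Tick events are disabled, and the construction script only calls its parent.
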(event EventBeginPlay
  (|CallParentFunction) ; This node is disabled and will not be called.\nDrag off pins to build functionality.
)

(event Collision|EventActorBeginOverlap
  (params (OtherActor :type Actor%20Object%20Reference))
  (|CallParentFunction OtherActor) ; This node is disabled and will not be called.\nDrag off pins to build functionality.
)

(event EventTick
  (params (DeltaSeconds :type Float%20%28single-precision%29))
  (|CallParentFunction DeltaSeconds) ; This node is disabled and will not be called.\nDrag off pins to build functionality.
)

(event EventPlayEquipSound
  (Audio|PlaySound2D "/Game/_Main/Sounds/WeaponSoundEffects/EquipWeaponitemSound.EquipWeaponitemSound" 1.0 1.0 0.0 0 0))

(event EventHandleAnimation
  (Components|Animation|PlayAnimation (Variables|Default|GetWeaponModel) "/Game/_Main/Models/WeaponModels/newrifletest/Animations/FireRifleAnimation_Rifle_SK_Fire.FireRifleAnimation_Rifle_SK_Fire" false))

(fn ConstructionScript
  (|CallParentFunction))