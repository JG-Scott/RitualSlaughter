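; Cultist enemy Blueprint that performs a melee-style montage attack and can rouse nearby enemies when alerted.
; Attack deals damage at an arrow on a montage notify and signals attack end on completion.
; Damage, death and one-time player-spotted sounds play with random pitch, reusing dog and Wendigo audio assets.
; A one-shot group alert switches enemies overlapping AlertSphere to attacking or investigating through their AI controllers, skipping those already in that state.
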(event Custom|AlertSurroundings
  (params (PlayerLocation :type Vector) (StateToSwapTo :type Enum_EnemyState%20Enum :default "NewEnumerator0") (AttackObject :type Actor%20Object%20Reference))
  (CallFunction|AlertGroupFunction PlayerLocation StateToSwapTo StateToSwapTo AttackObject))

(event EventBeginPlay)

(event Collision|EventActorBeginOverlap
  (params (OtherActor :type Actor%20Object%20Reference)))

(event EventTick
  (params (DeltaSeconds :type Float%20%28single-precision%29)))

(event EventAttack
  (Animation|Montage|PlayMontage (Variables|Character|GetMesh) "/Game/_Main/Models/RoughModels/Cultist/Animations/AM_CultistAttack.AM_CultistAttack"
    (:OnCompleted
      (Default|CallOnAttackEnd))
    (:OnNotifyBegin
      (CallFunction|DealDamageatArrow))))

(event EventPlayDamageSound
  (Audio|PlaySoundatLocation "/Game/_Main/Sounds/EnemySounds/DogSounds/Damage/DogDamageSoundCue.DogDamageSoundCue" (Transformation|GetActorLocation) "0, 0, 0" 1.0 (Math|Random|RandomFloatinRange 0.7 1.3) 0.0 "/Game/_Main/Models/RoughModels/DeerMan/Animations/Wendigo_WalkingAttenuation.Wendigo_WalkingAttenuation" 0 0 0))

(event EventPlayDeathSound
  (Audio|PlaySoundatLocation "/Game/_Main/Sounds/EnemySounds/DogSounds/dogdeath.dogdeath" (Transformation|GetActorLocation) "0, 0, 0" 1.0 (Math|Random|RandomFloatinRange 0.8 1.1) 0.0 "/Game/_Main/Models/RoughModels/DeerMan/Animations/Wendigo_WalkingAttenuation.Wendigo_WalkingAttenuation" 0 0 0))

(event EventPlayPlayerSpottedSound
  (Utilities|FlowControl|DoOnce false
    (:Completed
      (Audio|PlaySoundatLocation "/Game/_Main/Sounds/EnemySounds/WendigoSounds/Screams/Scream1.Scream1" (Transformation|GetActorLocation) "0, 0, 0" 1.0 (Math|Random|RandomFloatinRange 0.8 1.1) 0.0 "/Game/_Main/Models/RoughModels/DeerMan/Animations/Wendigo_WalkingAttenuation.Wendigo_WalkingAttenuation" 0 0 0))))

(fn ConstructionScript
  (|CallParentFunction))

(fn AlertGroupFunction
  (params (Location :type Vector) (InByte :type Byte) (Selection :type Enum_EnemyState%20Enum :default "NewEnumerator0") (AttackTarget :type Actor%20Object%20Reference))
  (if (not (Variables|Default|GetHasAlertedBefore))
    (Variables|Default|SetHasAlertedBefore true)
    (for _array_element (Collision|GetOverlappingActors (Variables|Default|GetAlertSphere) "/Game/_Main/Enemies/Rough/BP_EnemyBase.BP_EnemyBase_C" :!class /Script/Engine.PrimitiveComponent)
      (bind _asaic_enemy_base (Utilities|Casting|CastToAIC_Enemy_Base (AI|GetAIController _array_element)))
      (if (!= (Class|BlackboardComponent|GetValueasEnum (AI|GetBlackboard _asaic_enemy_base) (Variables|/Game/_Main/Enemies/AI/AIC_Enemy_Base.AIC_Enemy_Base_C|GetState _asaic_enemy_base)) (Math|Conversions|ToInteger(Byte) InByte))
        (switch Utilities|FlowControl|Switch|SwitchonEnum_EnemyState Selection
          (:NewEnumerator3
            (Default|SetStateasAttacking _asaic_enemy_base AttackTarget))
          (:NewEnumerator4
            (Default|SetStateasInvestigating _asaic_enemy_base Location)))))))