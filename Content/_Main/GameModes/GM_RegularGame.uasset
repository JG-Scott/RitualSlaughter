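; GM_RegularGame is the regular game mode, coordinating enemy spawners, altar destruction progress and light color.
; Events enable spawners, raise their enemy caps, or top them up to the cap with delayed random spawns before disabling them.
; Each destroyed altar increments a count and stops spawners; the five-altar ending only prints placeholder messages.
; A toggle switches lights between red and white, while both music events are empty stubs.
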(event Custom|AltarDestroyed
  (bind _result (Math|Integer|IncrementInt (Variables|Default|GetAltarsDestroyedCount))
    (:%20%20
      (CallFunction|StopSpawners)
      (if (>= _result 5)
        (Development|PrintString "Kill Horde")
        (Development|PrintString "End Game")))))

(event Custom|Stop%20Spawners
  (for _array_element (Variables|Default|GetSpawners)
    (if (<= (Variables|/Game/_Main/Props/EnemySpawner/BP_EnemySpawner.BP_EnemySpawner_C|GetCurrentEnemyAmount _array_element) (Variables|/Game/_Main/Props/EnemySpawner/BP_EnemySpawner.BP_EnemySpawner_C|GetMaximumEnemyAmount _array_element))
      (for _index (range 0 (- (Variables|/Game/_Main/Props/EnemySpawner/BP_EnemySpawner.BP_EnemySpawner_C|GetMaximumEnemyAmount _array_element) (Variables|/Game/_Main/Props/EnemySpawner/BP_EnemySpawner.BP_EnemySpawner_C|GetCurrentEnemyAmount _array_element)))
        (Utilities|FlowControl|Delay 0.5)
        (Default|SpawnRandomEnemy _array_element)))
    (Variables|/Game/_Main/Props/EnemySpawner/BP_EnemySpawner.BP_EnemySpawner_C|SetCanSpawnEnemies _array_element false)))

(event Custom|Start%20Spawners
  (for _array_element (Variables|Default|GetSpawners)
    (Variables|/Game/_Main/Props/EnemySpawner/BP_EnemySpawner.BP_EnemySpawner_C|SetCanSpawnEnemies _array_element true)))

(event Custom|IncreaseSpawners
  (for _array_element (Variables|Default|GetSpawners)
    (Variables|/Game/_Main/Props/EnemySpawner/BP_EnemySpawner.BP_EnemySpawner_C|SetMaximumEnemyAmount _array_element (+ (Variables|/Game/_Main/Props/EnemySpawner/BP_EnemySpawner.BP_EnemySpawner_C|GetMaximumEnemyAmount _array_element) 3))))

(event Custom|PlayAmbientMusic)

(event Custom|ToggleLights
  (params (IsRed :type Boolean))
  (for _array_element (Variables|Default|GetLights)
    (if IsRed
      (Rendering|Components|Light|SetLightColor (Variables|/Script/Engine.Light|GetLightComponent _array_element) "(R=1.000000,G=0.000000,B=0.013080,A=1.000000)" true)
      (else
        (Rendering|Components|Light|SetLightColor (Variables|/Script/Engine.Light|GetLightComponent _array_element) "(R=1.000000,G=1.000000,B=1.000000,A=1.000000)" true)))))

(event Custom|PlayChaseMusic)

(event EventBeginPlay)

(event EventTick
  (params (DeltaSeconds :type Float%20%28single-precision%29)))

(fn ConstructionScript)