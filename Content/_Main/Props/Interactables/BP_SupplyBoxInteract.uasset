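; Supply box interactable that bursts open and scatters random item drops when the player interacts with it.
; Interact plays the open sound and a scaled-up Niagara blood explosion at the box location, then destroys the actor after spawning the loot.
; Drops are picked at random from ItemPool, with the loop count rolled between the minimum and maximum drop amounts.
; The random index range includes the array length, so a pick can land past the last entry.
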(event EventBeginPlay
  (|CallParentFunction) ; This node is disabled and will not be called.\nDrag off pins to build functionality.
)

(event Collision|EventActorBeginOverlap
  (params (OtherActor :type Actor%20Object%20Reference))
  (|CallParentFunction OtherActor) ; This node is disabled and will not be called.\nDrag off pins to build functionality.
)

(event EventTick
  (params (DeltaSeconds :type Float%20%28single-precision%29))
  (|CallParentFunction DeltaSeconds) ; This node is disabled and will not be called.\nDrag off pins to build functionality.
)

(event EventInteract
  (params (CharacterPickingUp :type BP%20First%20Person%20Character%20Object%20Reference) (ActionValue :type Boolean))
  (bind _returnvalue (Transformation|GetActorLocation))
  (Development|PrintString "this is playing once")
  (Audio|PlaySoundatLocation "/Game/_Main/Sounds/SupplyCrateSounds/BoxOpen.BoxOpen" _returnvalue "0, 0, 0" 1.0 1.0 0.0 0 0 0 0)
  (Niagara|SpawnSystematLocation "/Game/_Main/ParticleEffects/ThrowableItemParticles/NS_BloodExplosion1.NS_BloodExplosion1" _returnvalue "0, 0, 0" "2.000000,2.000000,2.000000")
  (for _index (range 0 (Math|Random|RandomIntegerinRange (Variables|Default|GetMinItemDropAmount) (Variables|Default|GetMaxItemDropAmount)))
    (Game|SpawnActorfromClass (Utilities|Array|Get(acopy) (Variables|Default|GetItemPool) (Math|Random|RandomIntegerinRange 0 (Utilities|Array|Length (Variables|Default|GetItemPool)))) (Math|Transform|MakeTransform (Transformation|GetActorLocation) "0, 0, 0" "1.000000,1.000000,1.000000") "Undefined" "MultiplyWithRoot" 0 0))
  (Development|PrintString "destroy actor")
  (Actor|DestroyActor))

(fn ConstructionScript
  (|CallParentFunction))