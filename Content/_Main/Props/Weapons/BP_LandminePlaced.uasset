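; Placed landmine prop that beeps and flashes its point light on a repeating interval while waiting for an enemy.
; An overlap from a BP_EnemyBase triggers a one-second delayed explosion with effects and full radial damage credited to the first player's controller.
; The blast also calls Explode on landmines within a larger radius, creating staggered chain reactions, with a HasExploded flag preventing repeat detonation.
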(event OnComponentBeginOverlap(SphereOverlapCollision)
  (params (OverlappedComponent :type Primitive%20Component%20Object%20Reference) (OtherActor :type Actor%20Object%20Reference) (OtherComp :type Primitive%20Component%20Object%20Reference) (OtherBodyIndex :type Integer) (bFromSweep :type Boolean) (SweepResult :type Hit%20Result%20Structure%20%28by%20ref%29))
  (Utilities|Casting|CastToBP_EnemyBase OtherActor)
  (CallFunction|Explode))

(event Custom|ToggleLight
  (Rendering|Components|Light|SetIntensity (Variables|Default|GetPointLight) 1e+02)
  (Utilities|FlowControl|Delay 0.2)
  (Rendering|Components|Light|SetIntensity (Variables|Default|GetPointLight) 0.0))

(event Custom|Explode
  (bind _returnvalue (Transformation|GetActorLocation))
  (bind _returnvalue_2 (Transformation|GetActorLocation))
  (Utilities|FlowControl|Delay 1.0)
  (if (not (Variables|Default|GetHasExploded))
    (Variables|Default|SetHasExploded true)
    (Effects|SpawnEmitteratLocation "/Game/StarterContent/Particles/P_Explosion.P_Explosion" _returnvalue "0, 0, 0" "5.000000,5.000000,5.000000")
    (Audio|SpawnSoundatLocation "/Game/MilitaryWeapDark/Sound/RocketLauncher/wavs/RocketLauncher_Explosion01.RocketLauncher_Explosion01" _returnvalue "0, 0, 0" 1.0 1.0 0.0 0 0)
    (Game|Damage|ApplyRadialDamage (Variables|Default|GetExplosionDamage) _returnvalue_2 5e+02 0 0 self (Game|GetInstigatorController (Game|GetPlayerCharacter 0)) true "ECC_Visibility")
    (bind _outactors (Collision|SphereOverlapActors _returnvalue_2 7.5e+02 (Utilities|Array|MakeArray "ObjectTypeQuery2") "BP_LandminePlaced_C"))
    (for _array_element _outactors
      (Utilities|IsValid _array_element
        (:Is%20Valid
          (bind _asbp_landmine_placed (Utilities|Casting|CastToBP_LandminePlaced _array_element))
          (Utilities|IsValid _asbp_landmine_placed
            (:Is%20Valid
              (CallFunction|Explode _asbp_landmine_placed))))))
    (Actor|DestroyActor)))

(event EventBeginPlay
  (Audio|PlaySoundatLocation "/Game/_Main/Sounds/WeaponSoundEffects/landmineUseSoundEffect.landmineUseSoundEffect" (Transformation|GetActorLocation self) "0, 0, 0" 1.0 1.0 0.0 0 0 0 0)
  (Variables|Default|SetCurrentBeepTime (Variables|Default|GetBeepInterval)))

(event EventTick
  (params (DeltaSeconds :type Float%20%28single-precision%29))
  (bind _output_get (Variables|Default|SetCurrentBeepTime (- (Variables|Default|GetCurrentBeepTime) DeltaSeconds)))
  (if (<= _output_get 0.0)
    (Audio|PlaySoundatLocation "/Game/_Main/Sounds/WeaponSoundEffects/LandmineBeep.LandmineBeep" (Transformation|GetActorLocation self) "0, 0, 0" 1.0 1.0 0.0 "/Game/_Main/Models/RoughModels/DeerMan/Animations/Wendigo_WalkingAttenuation.Wendigo_WalkingAttenuation" 0 0 0)
    (Variables|Default|SetCurrentBeepTime (Variables|Default|GetBeepInterval))
    (CallFunction|ToggleLight)))

(fn ConstructionScript)