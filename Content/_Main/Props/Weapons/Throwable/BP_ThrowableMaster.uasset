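; BP_ThrowableMaster is a thrown weapon projectile, apparently a base for throwables, that spins, deals damage and destroys itself on impact.
; A timeline started on BeginPlay rotates the Weapon component, with an event available to stop it.
; Sphere overlaps with anything but BP_FirstPersonCharacter apply point damage credited to the player.
; Both those overlaps and solid box hits (guarded by DoOnce, no damage) spawn blood-explosion particles and sound, then destroy the actor.
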(event OnComponentBeginOverlap(SphereOverlapCollision)
  (params (OverlappedComponent :type Primitive%20Component%20Object%20Reference) (OtherActor :type Actor%20Object%20Reference) (OtherComp :type Primitive%20Component%20Object%20Reference) (OtherBodyIndex :type Integer) (bFromSweep :type Boolean) (SweepResult :type Hit%20Result%20Structure%20%28by%20ref%29))
  (bind (_bblockinghit _binitialoverlap _time _distance _location _impactpoint _normal _impactnormal _physmat _hitactor) (Collision|BreakHitResult SweepResult))
  (bind _boxsolidcollision (Variables|Default|GetBoxSolidCollision))
  (bind _returnvalue (Transformation|GetWorldLocation _boxsolidcollision))
  ;[1 1 1] Apply Damage To Damageable Objects On Impact
  (Utilities|Casting|CastToBP_FirstPersonCharacter OtherActor
    (:CastFailed
      (Game|Damage|ApplyPointDamage _hitactor (Variables|Default|GetThrownDamage) _location SweepResult (Game|GetInstigatorController (Game|GetPlayerCharacter 0)) self "/Script/Engine.DamageType")
      ;[1 1 1] Spawn Impact Particle System At Location
      (Niagara|SpawnSystematLocation "/Game/_Main/ParticleEffects/ThrowableItemParticles/NS_BloodExplosion1.NS_BloodExplosion1" _returnvalue)
      (Audio|SpawnSoundatLocation "/Game/MilitaryWeapSilver/Sound/Rifle/Wavs/RifleA_Fire01.RifleA_Fire01" _returnvalue "0, 0, 0" 0.5 1.0 0.0 0 0)
      (Actor|DestroyActor))))

(event OnComponentHit(BoxSolidCollision)
  (params (HitComponent :type Primitive%20Component%20Object%20Reference) (OtherActor :type Actor%20Object%20Reference) (OtherComp :type Primitive%20Component%20Object%20Reference) (NormalImpulse :type Vector :default "0, 0, 0") (Hit :type Hit%20Result%20Structure%20%28by%20ref%29))
  (bind _boxsolidcollision (Variables|Default|GetBoxSolidCollision))
  (bind _returnvalue (Transformation|GetWorldLocation _boxsolidcollision))
  ;[1 1 1] Spawn Impact Particle System At Location
  (Utilities|FlowControl|DoOnce false
    (:Completed
      (Niagara|SpawnSystematLocation "/Game/_Main/ParticleEffects/ThrowableItemParticles/NS_BloodExplosion1.NS_BloodExplosion1" _returnvalue)
      (Audio|SpawnSoundatLocation "/Game/MilitaryWeapSilver/Sound/Rifle/Wavs/RifleA_Fire01.RifleA_Fire01" _returnvalue "0, 0, 0" 0.5 1.0 0.0 0 0)
      (Actor|DestroyActor))))

(event Custom|BeginRotation
  (bind _newtrack_0 (Timeline|RotationTimeline Play)
    (:Update
      (Transformation|SetRelativeRotation (Variables|Default|GetWeapon) (Math|Rotator|Lerp(Rotator) "0, 0, 0" "1500.000000,1500.000000,0.000000" _newtrack_0) false false))))

(event Custom|stopRotation
  (bind _newtrack_0 (Timeline|RotationTimeline Stop)
    (:Update
      (Transformation|SetRelativeRotation (Variables|Default|GetWeapon) (Math|Rotator|Lerp(Rotator) "0, 0, 0" "1500.000000,1500.000000,0.000000" _newtrack_0) false false))))

(event EventBeginPlay
  (CallFunction|BeginRotation))

(event Collision|EventActorBeginOverlap
  (params (OtherActor :type Actor%20Object%20Reference)))

(fn ConstructionScript)