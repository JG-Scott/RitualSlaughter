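; Thrown grenade that explodes when its fuse timer runs out, building on inherited throwable behavior.
; Tick counts down the fuse, then spawns explosion particles and sound, enables query collision on ExplosionCircle and destroys the actor.
; Overlaps from that just-enabled volume, which is disabled at construction, apply point damage to anything except the first-person character, crediting player 0.
; Hits on the solid box only stop rotation, without detonating.
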(event OnComponentBeginOverlap(ExplosionCircle)
  (params (OverlappedComponent :type Primitive%20Component%20Object%20Reference) (OtherActor :type Actor%20Object%20Reference) (OtherComp :type Primitive%20Component%20Object%20Reference) (OtherBodyIndex :type Integer) (bFromSweep :type Boolean) (SweepResult :type Hit%20Result%20Structure%20%28by%20ref%29))
  (bind (_bblockinghit _binitialoverlap _time _distance _location _impactpoint _normal _impactnormal _physmat _hitactor) (Collision|BreakHitResult SweepResult))
  (Utilities|Casting|CastToBP_FirstPersonCharacter OtherActor
    (:CastFailed
      (Game|Damage|ApplyPointDamage _hitactor (Variables|Default|GetThrownDamage) _location SweepResult (Game|GetInstigatorController (Game|GetPlayerCharacter 0)) self "/Script/Engine.DamageType"))))

(event OnComponentHit(BoxSolidCollision)
  (params (HitComponent :type Primitive%20Component%20Object%20Reference) (OtherActor :type Actor%20Object%20Reference) (OtherComp :type Primitive%20Component%20Object%20Reference) (NormalImpulse :type Vector :default "0, 0, 0") (Hit :type Hit%20Result%20Structure%20%28by%20ref%29))
  (CallFunction|StopRotation))

(event EventBeginPlay
  (|CallParentFunction))

(event Collision|EventActorBeginOverlap
  (params (OtherActor :type Actor%20Object%20Reference))
  (|CallParentFunction OtherActor) ; This node is disabled and will not be called.\nDrag off pins to build functionality.
)

(event EventTick
  (params (DeltaSeconds :type Float%20%28single-precision%29))
  (bind _output_get (Variables|Default|SetFuse%20Timer (- (Variables|Default|GetFuse%20Timer) DeltaSeconds)))
  (if (<= _output_get 0.0)
    (Effects|SpawnEmitteratLocation "/Game/StarterContent/Particles/P_Explosion.P_Explosion" (Transformation|GetWorldLocation (Variables|Default|GetBoxSolidCollision)) "0, 0, 0" "5.000000,5.000000,5.000000")
    (Collision|SetCollisionEnabled (Variables|Default|GetExplosionCircle) "QueryOnly")
    (Audio|SpawnSoundatLocation "/Game/MilitaryWeapDark/Sound/RocketLauncher/wavs/RocketLauncher_Explosion01.RocketLauncher_Explosion01" "0, 0, 0" "0, 0, 0" 1.0 1.0 0.0 0 0)
    (Actor|DestroyActor)))

(fn ConstructionScript
  (|CallParentFunction)
  (Collision|SetCollisionEnabled (Variables|Default|GetExplosionCircle) "NoCollision")
  (Collision|SetCollisionEnabled (Variables|Default|GetSphereOverlapCollision) "NoCollision"))