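; BP_Cultist is an enemy that repeatedly AI-moves toward the player controller, restarting on success or failure until dead.
; Pawn sensing raises its walk speed on seeing a pawn.
; Point damage drains health; at zero it stops, spawns blood and giblet Niagara explosions, and destroys itself.
; The attack event is empty, with its montage and sphere-overlap damage logic left disconnected, as is a delayed-destroy branch.
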(event OnSeePawn(PawnSensing)
  (params (Pawn :type Pawn%20Object%20Reference))
  ;[1 1 1] Set run if player is near
  (Variables|/Script/Engine.CharacterMovementComponent|SetMaxWalkSpeed (Variables|Character|GetCharacterMovement) 3.6e+02))

(event Custom|RunToPlayer
  ;[1 1 1] Run to player logic
  (if (not (Variables|Default|GetIsDead?))
    (AI|AIMoveTo self "0, 0, 0" (Game|GetPlayerController 0) 4e+01 false
      (:OnSuccess
        _)
      (:OnFail
        _))
    (CallFunction|RuntoPlayer)))

(event Custom|AttackPlayer
  ;[1 1 1] Attack player animation logic
)

(event Custom|Death
  (bind _capsulecomponent (Variables|Collision|GetCapsuleComponent))
  (bind _returnvalue (Transformation|GetWorldLocation _capsulecomponent))
  ;[1 1 1] Death Logic
  (Variables|Default|SetIsDead? true)
  (Components|Movement|StopMovementImmediately (Variables|Character|GetCharacterMovement))
  (Niagara|SpawnSystematLocation "/Game/_Main/ParticleEffects/BloodSplatter/NS_BloodExplosion.NS_BloodExplosion" _returnvalue)
  (Niagara|SpawnSystematLocation "/Game/_Main/ParticleEffects/BloodSplatter/NS_GibletExplosion.NS_GibletExplosion" _returnvalue)
  (Actor|DestroyActor))

(event EventBeginPlay
  ;[1 1 1] Start run to player
  (CallFunction|RuntoPlayer))

(event Game|Damage|EventPointDamage
  (params (Damage :type Float%20%28single-precision%29) (DamageType :type Damage%20Type%20Object%20Reference) (HitLocation :type Vector :default "0, 0, 0") (HitNormal :type Vector :default "0, 0, 0") (HitComponent :type Primitive%20Component%20Object%20Reference) (BoneName :type Name :default "None") (ShotFromDirection :type Vector :default "0, 0, 0") (InstigatedBy :type Controller%20Object%20Reference) (DamageCauser :type Actor%20Object%20Reference) (HitInfo :type Hit%20Result%20Structure%20%28by%20ref%29))
  ;[1 1 1] HP Logic
  (if (not (Variables|Default|GetIsDead?))
    (bind _output_get (Variables|Default|SetHealth (- (Variables|Default|GetHealth) Damage)))
    (if (<= _output_get 0.0)
      (CallFunction|Death))))

(fn ConstructionScript)