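; Enemy spawner prop that, while enabled and under its population cap, periodically spawns a random dog, wendigo or cultist group at nearby navigable points.
; Spawns get the spawner's tag, team light color and a back-reference, with the first cultist in each group set as leader for the rest.
; In horde mode new enemies are set to attack the player.
; EnemyDeath decrements the count and notifies the game mode when the spawner is cleared.
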(event Custom|SpawnRandomEnemy
  (switch int (Math|Random|RandomIntegerinRange 0 2)
    (:0
      (CallFunction|SpawnScout))
    (:1
      (CallFunction|SpawnBigBoy))
    (:2
      (CallFunction|SpawnCultist))))

(event Custom|SpawnCultist
  (CallFunction|SpawnCultists))

(event Custom|SpawnScout
  (bind _randomlocation (Utilities|GetRandomLocation))
  (bind _returnvalue (Game|SpawnActorfromClass "/Game/_Main/Enemies/Rough/BP_DogEnemy.BP_DogEnemy_C" (Math|Transform|MakeTransform _randomlocation "0, 0, 0" "1.000000,1.000000,1.000000") "AdjustIfPossibleButAlwaysSpawn" "MultiplyWithRoot" 0 0))
  (Utilities|Array|Add (Variables|/Script/Engine.Actor|GetTags _returnvalue) (Variables|Default|GetEnemyTag))
  (Variables|/Game/_Main/Enemies/Rough/BP_EnemyBase.BP_EnemyBase_C|SetSpawner _returnvalue self)
  (Math|Integer|IncrementInt (Variables|Default|GetCurrentEnemyAmount)
    (:%20%20
      (Rendering|Components|Light|SetLightColor (Variables|/Game/_Main/Enemies/Rough/BP_EnemyBase.BP_EnemyBase_C|GetIdentifyingLight _returnvalue) (Variables|Default|GetTeamColor) true)
      (CallFunction|CheckifAltarBroken _returnvalue))))

(event Custom|CheckIfAltarBroken
  (params (NewParam :type BP%20Enemy%20Base%20Object%20Reference))
  (bind _asbp_first_person_game_mode (Utilities|Casting|CastToBP_FirstPersonGameMode (Game|GetGameMode)))
  (if (Variables|/Game/FirstPerson/Blueprints/BP_FirstPersonGameMode.BP_FirstPersonGameMode_C|GetIsInHordeMode _asbp_first_person_game_mode)
    (bind _asaic_enemy_base (Utilities|Casting|CastToAIC_Enemy_Base (AI|GetAIController NewParam)))
    (Default|SetStateasAttacking _asaic_enemy_base (Game|GetPlayerCharacter 0))))

(event Custom|SpawnBigBoy
  (bind _randomlocation (Utilities|GetRandomLocation))
  (bind _returnvalue (Game|SpawnActorfromClass "/Game/_Main/Enemies/Rough/BP_WendigoEnemy.BP_WendigoEnemy_C" (Math|Transform|MakeTransform _randomlocation "0, 0, 0" "1.000000,1.000000,1.000000") "AdjustIfPossibleButAlwaysSpawn" "MultiplyWithRoot" 0 0))
  (Utilities|Array|Add (Variables|/Script/Engine.Actor|GetTags _returnvalue) (Variables|Default|GetEnemyTag))
  (Variables|/Game/_Main/Enemies/Rough/BP_EnemyBase.BP_EnemyBase_C|SetSpawner _returnvalue self)
  (Rendering|Components|Light|SetLightColor (Variables|/Game/_Main/Enemies/Rough/BP_EnemyBase.BP_EnemyBase_C|GetIdentifyingLight _returnvalue) (Variables|Default|GetTeamColor) true)
  (Math|Integer|IncrementInt (Variables|Default|GetCurrentEnemyAmount)
    (:%20%20
      (CallFunction|CheckifAltarBroken _returnvalue))))

(event Custom|EnemyDeath
  (bind _result (Math|Integer|DecrementInt (Variables|Default|GetCurrentEnemyAmount))
    (:%20%20
      (if (<= _result 0)
        (bind _asbp_first_person_game_mode (Utilities|Casting|CastToBP_FirstPersonGameMode (Game|GetGameMode)))
        (Default|SpawnerCleared _asbp_first_person_game_mode)))))

(event EventBeginPlay
  (Variables|Default|SetSpawnTimerOriginal (Variables|Default|GetSpawnTimer)))

(event Collision|EventActorBeginOverlap
  (params (OtherActor :type Actor%20Object%20Reference)))

(event EventTick
  (params (DeltaSeconds :type Float%20%28single-precision%29))
  (if (Variables|Default|GetCanSpawnEnemies)
    (if (< (Variables|Default|GetCurrentEnemyAmount) (Variables|Default|GetMaximumEnemyAmount))
      (bind _output_get (Variables|Default|SetSpawnTimer (- (Variables|Default|GetSpawnTimer) DeltaSeconds)))
      (if (<= _output_get 0.0)
        (Variables|Default|SetSpawnTimer (Variables|Default|GetSpawnTimerOriginal))
        (CallFunction|SpawnRandomEnemy)))))

(fn ConstructionScript)

(fn SpawnCultists
  (bind _minimumcultistgroupamount (Variables|Default|GetMinimumCultistGroupAmount))
  (bind _maximumcultistgroupamount (Variables|Default|GetMaximumCultistGroupAmount))
  (bind _returnvalue (Math|Random|RandomIntegerinRange _minimumcultistgroupamount _maximumcultistgroupamount))
  (if (> (+ _returnvalue (Variables|Default|GetCurrentEnemyAmount)) (Variables|Default|GetMaximumEnemyAmount))
    (for _index (range 0 (- (Variables|Default|GetMaximumEnemyAmount) (Variables|Default|GetCurrentEnemyAmount)))
      (if (== _index 0)
        (bind _randomlocation (Utilities|GetRandomLocation))
        (bind _returnvalue_2 (Game|SpawnActorfromClass "/Game/_Main/Enemies/Rough/BP_CultistEnemy.BP_CultistEnemy_C" (Math|Transform|MakeTransform _randomlocation "0, 0, 0" "1.000000,1.000000,1.000000") "AdjustIfPossibleButAlwaysSpawn" "MultiplyWithRoot" 0 0))
        (Utilities|Array|Add (Variables|/Script/Engine.Actor|GetTags _returnvalue_2) (Variables|Default|GetEnemyTag))
        (Variables|/Game/_Main/Enemies/Rough/BP_EnemyBase.BP_EnemyBase_C|SetSpawner _returnvalue_2 self)
        (Rendering|Components|Light|SetLightColor (Variables|/Game/_Main/Enemies/Rough/BP_EnemyBase.BP_EnemyBase_C|GetIdentifyingLight _returnvalue_2) (Variables|Default|GetTeamColor) true)
        (LocalVariables|SetLeader _returnvalue_2)
        (Math|Integer|IncrementInt (Variables|Default|GetCurrentEnemyAmount)
          (:%20%20
            (CallFunction|CheckifAltarBroken _returnvalue_2)))
        (else
          (bind _randomlocation_2 (Utilities|GetRandomLocation))
          (bind _returnvalue_3 (Game|SpawnActorfromClass "/Game/_Main/Enemies/Rough/BP_CultistEnemy.BP_CultistEnemy_C" (Math|Transform|MakeTransform _randomlocation_2 "0, 0, 0" "1.000000,1.000000,1.000000") "AdjustIfPossibleButAlwaysSpawn" "MultiplyWithRoot" 0 0))
          (Utilities|Array|Add (Variables|/Script/Engine.Actor|GetTags _returnvalue_3) (Variables|Default|GetEnemyTag))
          (Rendering|Components|Light|SetLightColor (Variables|/Game/_Main/Enemies/Rough/BP_EnemyBase.BP_EnemyBase_C|GetIdentifyingLight _returnvalue_3) (Variables|Default|GetTeamColor) true)
          (Variables|/Game/_Main/Enemies/Rough/BP_EnemyBase.BP_EnemyBase_C|SetSpawner _returnvalue_3 self)
          (bind _asaic_horde_filler (Utilities|Casting|CastToAIC_HordeFiller (AI|GetAIController _returnvalue_3)))
          (Default|SetLeader _asaic_horde_filler (LocalVariables|GetLeader))
          (Math|Integer|IncrementInt (Variables|Default|GetCurrentEnemyAmount)
            (:%20%20
              (CallFunction|CheckifAltarBroken _returnvalue_3))))))
    (else
      (for _index_2 (range 0 _returnvalue)
        (if (== _index_2 0)
          (bind _randomlocation_3 (Utilities|GetRandomLocation))
          (bind _returnvalue_4 (Game|SpawnActorfromClass "/Game/_Main/Enemies/Rough/BP_CultistEnemy.BP_CultistEnemy_C" (Math|Transform|MakeTransform _randomlocation_3 "0, 0, 0" "1.000000,1.000000,1.000000") "AdjustIfPossibleButAlwaysSpawn" "MultiplyWithRoot" 0 0))
          (Utilities|Array|Add (Variables|/Script/Engine.Actor|GetTags _returnvalue_4) (Variables|Default|GetEnemyTag))
          (Variables|/Game/_Main/Enemies/Rough/BP_EnemyBase.BP_EnemyBase_C|SetSpawner _returnvalue_4 self)
          (Rendering|Components|Light|SetLightColor (Variables|/Game/_Main/Enemies/Rough/BP_EnemyBase.BP_EnemyBase_C|GetIdentifyingLight _returnvalue_4) (Variables|Default|GetTeamColor) true)
          (LocalVariables|SetLeader _returnvalue_4)
          (Math|Integer|IncrementInt (Variables|Default|GetCurrentEnemyAmount)
            (:%20%20
              (CallFunction|CheckifAltarBroken _returnvalue_4)))
          (else
            (bind _randomlocation_4 (Utilities|GetRandomLocation))
            (bind _returnvalue_5 (Game|SpawnActorfromClass "/Game/_Main/Enemies/Rough/BP_CultistEnemy.BP_CultistEnemy_C" (Math|Transform|MakeTransform _randomlocation_4 "0, 0, 0" "1.000000,1.000000,1.000000") "AdjustIfPossibleButAlwaysSpawn" "MultiplyWithRoot" 0 0))
            (Utilities|Array|Add (Variables|/Script/Engine.Actor|GetTags _returnvalue_5) (Variables|Default|GetEnemyTag))
            (Rendering|Components|Light|SetLightColor (Variables|/Game/_Main/Enemies/Rough/BP_EnemyBase.BP_EnemyBase_C|GetIdentifyingLight _returnvalue_5) (Variables|Default|GetTeamColor) true)
            (Variables|/Game/_Main/Enemies/Rough/BP_EnemyBase.BP_EnemyBase_C|SetSpawner _returnvalue_5 self)
            (bind _asaic_horde_filler_2 (Utilities|Casting|CastToAIC_HordeFiller (AI|GetAIController _returnvalue_5)))
            (Default|SetLeader _asaic_horde_filler_2 (LocalVariables|GetLeader))
            (Math|Integer|IncrementInt (Variables|Default|GetCurrentEnemyAmount)
              (:%20%20
                (CallFunction|CheckifAltarBroken _returnvalue_5)))))))))