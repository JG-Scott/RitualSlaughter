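; BP_HealthKit is a health kit item that heals the player when used, with fire and equip events like a weapon.
; TriggerFire plays a use sound, calls DestroyAndSpawnNewWeapon on the first-person player character, then adds HealAmount to its CurrentHealth, capped at MaxHealth.
; PlayEquipSound plays an item equip sound, while BeginPlay, overlap and Tick are disabled stubs.
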(event EventBeginPlay
  (|CallParentFunction) ; This node is disabled and will not be called.\nDrag off pins to build functionality.
)

(event Collision|EventActorBeginOverlap
  (params (OtherActor :type Actor%20Object%20Reference))
  (|CallParentFunction OtherActor) ; This node is disabled and will not be called.\nDrag off pins to build functionality.
)

(event EventTick
  (params (DeltaSeconds :type Float%20%28single-precision%29))
  (|CallParentFunction DeltaSeconds) ; This node is disabled and will not be called.\nDrag off pins to build functionality.
)

(event EventTriggerFire
  (params (Release :type Boolean) (PlayerRef :type Actor%20Object%20Reference) (CameraLocation :type Vector :default "0, 0, 0") (CameraRotation :type Rotator :default "0, 0, 0"))
  (Audio|PlaySound2D "/Game/_Main/Sounds/WeaponSoundEffects/HealthKitUse.HealthKitUse" 1.0 1.0 0.0 0 0)
  (bind _asbp_first_person_character (Utilities|Casting|CastToBP_FirstPersonCharacter (Game|GetPlayerCharacter 0)))
  (Default|DestroyandSpawnNewWeapon _asbp_first_person_character)
  (if (> (+ (Variables|/Game/FirstPerson/Blueprints/BP_FirstPersonCharacter.BP_FirstPersonCharacter_C|GetCurrentHealth _asbp_first_person_character) (Variables|Default|GetHealAmount)) (Variables|/Game/FirstPerson/Blueprints/BP_FirstPersonCharacter.BP_FirstPersonCharacter_C|GetMaxHealth _asbp_first_person_character))
    (Variables|/Game/FirstPerson/Blueprints/BP_FirstPersonCharacter.BP_FirstPersonCharacter_C|SetCurrentHealth _asbp_first_person_character (Variables|/Game/FirstPerson/Blueprints/BP_FirstPersonCharacter.BP_FirstPersonCharacter_C|GetMaxHealth _asbp_first_person_character))
    (else
      (Variables|/Game/FirstPerson/Blueprints/BP_FirstPersonCharacter.BP_FirstPersonCharacter_C|SetCurrentHealth _asbp_first_person_character (+ (Variables|/Game/FirstPerson/Blueprints/BP_FirstPersonCharacter.BP_FirstPersonCharacter_C|GetCurrentHealth _asbp_first_person_character) (Variables|Default|GetHealAmount))))))

(event EventPlayEquipSound
  (Audio|PlaySound2D "/Game/_Main/Sounds/WeaponSoundEffects/ItemEquip.ItemEquip" 1.0 1.0 0.0 0 0))

(fn ConstructionScript
  (|CallParentFunction))