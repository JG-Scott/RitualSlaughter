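; BP_WendigoEnemy is a Wendigo enemy Blueprint that rouses nearby enemies when it raises an alert.
; AlertSurroundings fires only once, gathering BP_EnemyBase actors inside its AlertSphere.
; Their AI controllers switch to attacking the given target or investigating the given location, unless hostile to the Wendigo or already in that state.
; SetMovementSpeed is a stub returning zero, and the light-colour call is unconnected.
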(event Custom|AlertSurroundings
  (params (PlayerLocation :type Vector) (StateToSwapTo :type Enum_EnemyState%20Enum :default "NewEnumerator0") (AttackObject :type Actor%20Object%20Reference))
  (CallFunction|AlertSurroundingsFunction PlayerLocation StateToSwapTo StateToSwapTo AttackObject))

(event EventBeginPlay
  (|CallParentFunction))

(event Collision|EventActorBeginOverlap
  (params (OtherActor :type Actor%20Object%20Reference)))

(event EventTick
  (params (DeltaSeconds :type Float%20%28single-precision%29)))

(fn ConstructionScript
  (|CallParentFunction))

(fn SetMovementSpeed
  (params (Movement%20Type :type Enum_EnemyMovementType%20Enum :default "NewEnumerator0"))
  (return 0.0))

(fn AlertSurroundingsFunction
  (params (Location :type Vector) (InByte :type Byte) (Selection :type Enum_EnemyState%20Enum :default "NewEnumerator0") (AttackTarget :type Actor%20Object%20Reference))
  (if (not (Variables|Default|GetHasAlertedBefore))
    (Variables|Default|SetHasAlertedBefore true)
    (for _array_element (Collision|GetOverlappingActors (Variables|Default|GetAlertSphere) "/Game/_Main/Enemies/Rough/BP_EnemyBase.BP_EnemyBase_C" :!class /Script/Engine.PrimitiveComponent)
      (bind _asaic_enemy_base (Utilities|Casting|CastToAIC_Enemy_Base (AI|GetAIController _array_element)))
      (LocalVariables|SetEnemyToAlert _asaic_enemy_base)
      (if (and (!= (Class|BlackboardComponent|GetValueasEnum (AI|GetBlackboard (LocalVariables|GetEnemyToAlert)) (Variables|/Game/_Main/Enemies/AI/AIC_Enemy_Base.AIC_Enemy_Base_C|GetState (LocalVariables|GetEnemyToAlert))) (Math|Conversions|ToInteger(Byte) Selection)) (not (Default|IsEnemyTeam (LocalVariables|GetEnemyToAlert) self)))
        (switch Utilities|FlowControl|Switch|SwitchonEnum_EnemyState Selection
          (:NewEnumerator3
            (Default|SetStateasAttacking (LocalVariables|GetEnemyToAlert) AttackTarget))
          (:NewEnumerator4
            (Default|SetStateasInvestigating (LocalVariables|GetEnemyToAlert) Location)))))))