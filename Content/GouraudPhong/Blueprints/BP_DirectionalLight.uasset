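; Directional light actor that feeds global lighting values to materials through the MPC_GlobalLighting parameter collection.
; UpdateLight runs on construction and BeginPlay, writing directional, ambient and specular colours to the collection.
; It clamps LightDirection per axis, uses it as the DirectionalLight component's relative location, and writes it scaled down and multiplied by Brightness as DirectionalVector, so intensity is carried in the vector's length.
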(event EventBeginPlay
  (CallFunction|UpdateLight))

(fn ConstructionScript
  (CallFunction|UpdateLight))

(fn UpdateLight
  (bind _lightdirection (Variables|DirectionalLight|GetLightDirection))
  (bind _returnvalue (Math|Float|Clamp(Float) (.x _lightdirection) -2.5e+02 2.5e+02))
  (bind _returnvalue_2 (Math|Float|Clamp(Float) (.y _lightdirection) -2.5e+02 2.5e+02))
  (bind _returnvalue_3 (Math|Float|Clamp(Float) (.z _lightdirection) -2.5e+02 2.5e+02))
  (bind _returnvalue_4 (Math|Vector|MakeVector _returnvalue _returnvalue_2 _returnvalue_3))
  ;[1 1 1] Directional Light
  (Rendering|Material|SetVectorParameterValue "/Game/GouraudPhong/Materials/MPC_GlobalLighting.MPC_GlobalLighting" "DirectionalColour" (Variables|DirectionalLight|GetLightColour) :!class /Script/Engine.KismetMaterialLibrary)
  (Rendering|Material|SetVectorParameterValue "/Game/GouraudPhong/Materials/MPC_GlobalLighting.MPC_GlobalLighting" "AmbientColour" (Variables|DirectionalLight|GetAmbientColour) :!class /Script/Engine.KismetMaterialLibrary)
  (Rendering|Material|SetVectorParameterValue "/Game/GouraudPhong/Materials/MPC_GlobalLighting.MPC_GlobalLighting" "DirectionalSpecular" (Variables|DirectionalLight|GetSpecularColour) :!class /Script/Engine.KismetMaterialLibrary)
  (Transformation|SetRelativeLocation (Variables|Default|GetDirectionalLight) _returnvalue_4 false false)
  (Rendering|Material|SetVectorParameterValue "/Game/GouraudPhong/Materials/MPC_GlobalLighting.MPC_GlobalLighting" "DirectionalVector" (Math|Conversions|ToLinearColor(Vector) (* (/ _returnvalue_4 1e+02) (Variables|DirectionalLight|GetBrightness))) :!class /Script/Engine.KismetMaterialLibrary))