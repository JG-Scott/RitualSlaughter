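; Experimental custom shadow-map actor that uses a scene capture to view a list of shadow casters from a light direction.
; LightTransform derives a basis from LightVector to aim the capture, offset back from a target mesh's bounding sphere with an ortho width matching its diameter.
; BeginPlay and the construction script write the light-space parameters to MPC_Shadowmap for materials, but construction sets the collection's OrthoWidth to zero.
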(event EventBeginPlay
  (bind (_x _y _z) (CallFunction|LightTransform))
  (bind _scenecapturecomponent2d (Variables|Default|GetSceneCaptureComponent2D))
  (bind _smeshactor (Variables|Default|GetSMeshActor))
  (bind _staticmeshcomponent (Variables|/Script/Engine.StaticMeshActor|GetStaticMeshComponent _smeshactor))
  (bind (_origin _boxextent _sphereradius) (Collision|GetComponentBounds _staticmeshcomponent))
  (Transformation|SetWorldLocationAndRotation (Variables|Default|GetSceneCaptureComponent2D) (+ _origin (* _x (* _sphereradius -1.5))) (Math|Rotator|MakeRotfromXZ _x _z) false false)
  (bind _output_get (Variables|/Script/Engine.SceneCaptureComponent2D|SetOrthoWidth (Variables|Default|GetSceneCaptureComponent2D) (* (.SphereRadius (Collision|GetComponentBounds (Variables|/Script/Engine.StaticMeshActor|GetStaticMeshComponent (Variables|Default|GetSMeshActor)))) 2.0)))
  (Rendering|Material|SetVectorParameterValue "/Game/GouraudPhong/Experimental/Materials/MPC_Shadowmap.MPC_Shadowmap" "LightPosition" (Math|Conversions|ToLinearColor(Vector) (Transformation|GetWorldLocation _scenecapturecomponent2d)) :!class /Script/Engine.KismetMaterialLibrary)
  (Rendering|Material|SetVectorParameterValue "/Game/GouraudPhong/Experimental/Materials/MPC_Shadowmap.MPC_Shadowmap" "LightRightDirection" (Math|Conversions|ToLinearColor(Vector) (Math|Vector|GetRightVector _scenecapturecomponent2d)) :!class /Script/Engine.KismetMaterialLibrary)
  (Rendering|Material|SetVectorParameterValue "/Game/GouraudPhong/Experimental/Materials/MPC_Shadowmap.MPC_Shadowmap" "LightDirection" (Math|Conversions|ToLinearColor(Vector) (Math|Vector|GetForwardVector _scenecapturecomponent2d)) :!class /Script/Engine.KismetMaterialLibrary)
  (Rendering|Material|SetScalarParameterValue "/Game/GouraudPhong/Experimental/Materials/MPC_Shadowmap.MPC_Shadowmap" "OrthoWidth" _output_get :!class /Script/Engine.KismetMaterialLibrary)
  (Variables|/Script/Engine.SceneCaptureComponent|SetShowOnlyActors (Variables|Default|GetSceneCaptureComponent2D) (Variables|Default|GetShadowCasters)))

(fn ConstructionScript
  (bind (_x _y _z) (CallFunction|LightTransform))
  (bind _scenecapturecomponent2d (Variables|Default|GetSceneCaptureComponent2D))
  (bind _smeshactor (Variables|Default|GetSMeshActor))
  (bind _staticmeshcomponent (Variables|/Script/Engine.StaticMeshActor|GetStaticMeshComponent _smeshactor))
  (bind (_origin _boxextent _sphereradius) (Collision|GetComponentBounds _staticmeshcomponent))
  (Transformation|SetWorldLocationAndRotation (Variables|Default|GetSceneCaptureComponent2D) (+ _origin (* _x (* _sphereradius -1.5))) (Math|Rotator|MakeRotfromXZ _x _z) false false)
  (Variables|/Script/Engine.SceneCaptureComponent2D|SetOrthoWidth (Variables|Default|GetSceneCaptureComponent2D) (* (.SphereRadius (Collision|GetComponentBounds (Variables|/Script/Engine.StaticMeshActor|GetStaticMeshComponent (Variables|Default|GetSMeshActor)))) 2.0))
  (Rendering|Material|SetVectorParameterValue "/Game/GouraudPhong/Experimental/Materials/MPC_Shadowmap.MPC_Shadowmap" "LightPosition" (Math|Conversions|ToLinearColor(Vector) (Transformation|GetWorldLocation _scenecapturecomponent2d)) :!class /Script/Engine.KismetMaterialLibrary)
  (Rendering|Material|SetVectorParameterValue "/Game/GouraudPhong/Experimental/Materials/MPC_Shadowmap.MPC_Shadowmap" "LightRightDirection" (Math|Conversions|ToLinearColor(Vector) (Math|Vector|GetRightVector _scenecapturecomponent2d)) :!class /Script/Engine.KismetMaterialLibrary)
  (Rendering|Material|SetVectorParameterValue "/Game/GouraudPhong/Experimental/Materials/MPC_Shadowmap.MPC_Shadowmap" "LightDirection" (Math|Conversions|ToLinearColor(Vector) (Math|Vector|GetForwardVector _scenecapturecomponent2d)) :!class /Script/Engine.KismetMaterialLibrary)
  (Rendering|Material|SetScalarParameterValue "/Game/GouraudPhong/Experimental/Materials/MPC_Shadowmap.MPC_Shadowmap" "OrthoWidth" 0.0 :!class /Script/Engine.KismetMaterialLibrary)
  (Variables|/Script/Engine.SceneCaptureComponent|SetShowOnlyActors (Variables|Default|GetSceneCaptureComponent2D) (Variables|Default|GetShadowCasters)))

(fn LightTransform
  (bind _lightvector (Variables|Default|GetLightVector))
  (bind _returnvalue (Math|Vector|Normalize _lightvector))
  (bind _returnvalue_2 (* _lightvector "0, 0,-1.000000"))
  (bind _returnvalue_3 (Math|Vector|Normalize _returnvalue_2))
  (bind _returnvalue_4 (* _returnvalue _returnvalue_3))
  (bind _returnvalue_5 (Math|Vector|Normalize _returnvalue_4))
  (return _returnvalue (Math|Vector|Normalize (* _returnvalue _returnvalue_5)) _returnvalue_5))