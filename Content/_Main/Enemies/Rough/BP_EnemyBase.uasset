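; Base Wendigo-style enemy character with melee attack, health, death and movement helpers such as state switching, speed presets and random navmesh travel points.
; Attack montage notifies trigger a sphere overlap at an arrow, damaging the player and other enemies that lack its second actor tag.
; Incoming damage is reported to AI perception, plays a scream and flashes a point light.
; Death spawns blood and giblet Niagara effects, notifies its spawner and destroys the actor.
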(event Custom|PlayPlayerSpottedSound
  ;[1 0.8349 0.1142] Sound effects
  (Utilities|FlowControl|DoOnce false
    (:Completed
      (Audio|PlaySoundatLocation "/Game/_Main/Sounds/EnemySounds/WendigoSounds/Screams/Scream2.Scream2" (Transformation|GetActorLocation self) "0, 0, 0" 1.0 (Math|Random|RandomFloatinRange 0.8 1.1) 0.0 "/Game/_Main/Models/RoughModels/DeerMan/Animations/Wendigo_WalkingAttenuation.Wendigo_WalkingAttenuation" 0 0 0))))

(event Custom|PlayAttackSound
  ;[1 0.8349 0.1142] Sound effects
  (Audio|PlaySoundatLocation "/Game/_Main/Sounds/EnemySounds/WendigoSounds/WendigoAttack.WendigoAttack" (Transformation|GetActorLocation self) "0, 0, 0" 1.0 1.0 0.0 "/Game/_Main/Models/RoughModels/DeerMan/Animations/Wendigo_WalkingAttenuation.Wendigo_WalkingAttenuation" 0 0 0))

(event Custom|Death
  (bind _capsulecomponent (Variables|Collision|GetCapsuleComponent))
  (bind _returnvalue (Transformation|GetWorldLocation _capsulecomponent))
  ;[1 1 1] Death Logic
  (CallFunction|PlayDeathSound)
  (Variables|Default|SetIsDead? true)
  (Components|Movement|StopMovementImmediately (Variables|Character|GetCharacterMovement))
  (Niagara|SpawnSystematLocation "/Game/_Main/ParticleEffects/BloodSplatter/NS_BloodExplosion.NS_BloodExplosion" _returnvalue)
  (Niagara|SpawnSystematLocation "/Game/_Main/ParticleEffects/BloodSplatter/NS_GibletExplosion.NS_GibletExplosion" _returnvalue "0, 0, 0" "5.000000,5.000000,5.000000")
  (Default|EnemyDeath (Variables|Default|GetSpawner))
  (Actor|DestroyActor))

(event Custom|TogglePawnCollision
  (Collision|SetCollisionResponsetoChannel (Variables|Collision|GetCapsuleComponent) "ECC_Pawn" "ECR_Ignore"))

(event Custom|Attack
  ;[1 1 1] Attacking animation
  (Animation|Montage|PlayMontage (Variables|Character|GetMesh) "/Game/_Main/Models/RoughModels/DeerMan/Animations/Montage_WendigoEnemyAttackAnim.Montage_WendigoEnemyAttackAnim"
    (:OnCompleted
      (Default|CallOnAttackEnd))
    (:OnNotifyBegin
      (CallFunction|DealDamageatArrow))))

(event Custom|PlayDamageSound
  ;[1 0.8349 0.1142] Sound effects
  (Audio|PlaySoundatLocation "/Game/_Main/Sounds/EnemySounds/WendigoSounds/Screams/TakeDamageScream.TakeDamageScream" (Transformation|GetActorLocation self) "0, 0, 0" 1.0 (Math|Random|RandomFloatinRange 0.75 1.0) 0.0 "/Game/_Main/Models/RoughModels/DeerMan/Animations/Wendigo_WalkingAttenuation.Wendigo_WalkingAttenuation" 0 0 0))

(event Custom|PlayDeathSound
  ;[1 0.8349 0.1142] Sound effects
  (Audio|PlaySoundatLocation "/Game/_Main/Sounds/EnemySounds/WendigoSounds/Screams/littleScream.littleScream" (Transformation|GetActorLocation self) "0, 0, 0" 1.0 (Math|Random|RandomFloatinRange 0.8 1.1) 0.0 0 0 0 0))

(event Custom|ToggleDamageLight
  ;[1 1 1] Damage Indicator Light
  (Rendering|Components|Light|SetIntensity (Variables|Default|GetPointLight) 1e+03)
  (Utilities|FlowControl|Delay 0.1)
  (Rendering|Components|Light|SetIntensity (Variables|Default|GetPointLight) 0.0))

(event Game|Damage|EventAnyDamage
  (params (Damage :type Float%20%28single-precision%29) (DamageType :type Damage%20Type%20Object%20Reference) (InstigatedBy :type Controller%20Object%20Reference) (DamageCauser :type Actor%20Object%20Reference))
  ;[1 1 1] Take Damage Logic
  (Class|AISenseDamage|ReportDamageEvent self InstigatedBy Damage (Transformation|GetActorLocation InstigatedBy) "0, 0, 0" "None")
  (CallFunction|PlayDamageSound)
  (CallFunction|ToggleDamageLight)
  (if (not (Variables|Default|GetIsDead?))
    (bind _output_get (Variables|Default|SetHealth (- (Variables|Default|GetHealth) Damage)))
    (if (<= _output_get 0.0)
      (CallFunction|Death))))

(fn ConstructionScript)

(fn SwitchEnemyState
  (params (new%20state :type Enum_EnemyState%20Enum :default "NewEnumerator0"))
  (Variables|Enums|SetCurrentState new%20state))

(fn DealDamageatArrow
  (bind _array (Utilities|Array|MakeArray "ObjectTypeQuery3"))
  (bind _arrow1 (Variables|Default|GetArrow1))
  (bind _returnvalue (Transformation|GetWorldLocation _arrow1))
  (bind _outactors (Actor|GetAllActorsOfClasswithTag "BP_EnemyBase_C" (Utilities|Array|Get(acopy) (Variables|Actor|GetTags self) 1)))
  (Utilities|Array|Add _outactors self)
  (bind (_outactors_2 _returnvalue_2) (Collision|SphereOverlapActors _returnvalue 8e+01 _array "BP_EnemyBase_C" _outactors))
  (bind (_outactors_3 _returnvalue_3) (Collision|SphereOverlapActors _returnvalue 8e+01 _array "/Game/FirstPerson/Blueprints/BP_FirstPersonCharacter.BP_FirstPersonCharacter_C"))
  (for _array_element _outactors_3
    (Utilities|Array|Add _outactors_2 _array_element))
  (if (or _returnvalue_3 _returnvalue_2)
    (for _array_element_2 _outactors_2
      (if (not (Actor|ActorHasTag _array_element_2 (Utilities|Array|Get(acopy) (Variables|Actor|GetTags self) 1)))
        (Game|Damage|ApplyDamage _array_element_2 2e+01 (Game|GetInstigatorController) self)))))

(fn GetNewTravelLocation
  (bind _randomlocation (Class|NavigationSystemV1|GetRandomLocationinNavigableRadius (Transformation|GetActorLocation) (Variables|MovementVariables|GetMinimumTravelRadius) 0 0))
  (bind _randomlocation_2 (Class|NavigationSystemV1|GetRandomLocationinNavigableRadius _randomlocation (Variables|MovementVariables|GetTravelRadius) 0 0))
  (Collision|MultiLineTraceByChannel _randomlocation_2 (Math|Vector|MakeVector (.X (Math|Vector|BreakVector _randomlocation_2)) (.Y (Math|Vector|BreakVector _randomlocation_2)) -1e+04) "TraceTypeQuery1" false 0 "None" true "(R=1.000000,G=0.000000,B=0.000000,A=1.000000)" "(R=0.000000,G=1.000000,B=0.000000,A=1.000000)" 2.0)
  (bind _output_get (Variables|Default|SetCurrentTravelLocation _randomlocation_2))
  (return _output_get))

(fn SetMovementSpeed
  (params (Movement%20Type :type Enum_EnemyMovementType%20Enum :default "NewEnumerator0"))
  (bind _output_get (Variables|/Script/Engine.CharacterMovementComponent|SetMaxWalkSpeed (Variables|Character|GetCharacterMovement) (Utilities|Select :Index Movement%20Type :NewEnumerator0 0.0 :NewEnumerator1 6e+02 :NewEnumerator2 9e+02)))
  (return _output_get))