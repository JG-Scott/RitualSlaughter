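; Dog enemy character that bites the player and supplies its own roaming, movement speed and sounds.
; Attack plays a bite montage, dealing damage at an arrow on its notify and signalling attack end on completion.
; Helpers pick random navmesh travel points and map movement type to walk speed.
; Pitch-randomised damage, death and player-spotted sounds play, the last only once; an unconnected sphere-overlap damage check never runs.
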(event EventBeginPlay
  (|CallParentFunction) ; This node is disabled and will not be called.\nDrag off pins to build functionality.
)

(event Collision|EventActorBeginOverlap
  (params (OtherActor :type Actor%20Object%20Reference)))

(event EventTick
  (params (DeltaSeconds :type Float%20%28single-precision%29)))

(event EventAttack
  (Animation|Montage|PlayMontage (Variables|Character|GetMesh) "/Game/_Main/Models/RoughModels/Dog/animations/AM_DogBite.AM_DogBite"
    (:OnCompleted
      (Default|CallOnAttackEnd))
    (:OnNotifyBegin
      (CallFunction|DealDamageatArrow))))

(event EventPlayDeathSound
  (Audio|PlaySoundatLocation "/Game/_Main/Sounds/EnemySounds/DogSounds/dogdeath.dogdeath" (Transformation|GetActorLocation) "0, 0, 0" 1.0 (Math|Random|RandomFloatinRange 0.8 1.1) 0.0 "/Game/_Main/Models/RoughModels/DeerMan/Animations/Wendigo_WalkingAttenuation.Wendigo_WalkingAttenuation" 0 0 0))

(event EventPlayDamageSound
  (Audio|PlaySoundatLocation "/Game/_Main/Sounds/EnemySounds/DogSounds/Damage/DogDamageSoundCue.DogDamageSoundCue" (Transformation|GetActorLocation) "0, 0, 0" 1.0 (Math|Random|RandomFloatinRange 0.7 1.3) 0.0 "/Game/_Main/Models/RoughModels/DeerMan/Animations/Wendigo_WalkingAttenuation.Wendigo_WalkingAttenuation" 0 0 0))

(event EventPlayPlayerSpottedSound
  (Utilities|FlowControl|DoOnce false
    (:Completed
      (Audio|PlaySoundatLocation "/Game/_Main/Sounds/EnemySounds/DogSounds/dogplayerspottend.dogplayerspottend" (Transformation|GetActorLocation) "0, 0, 0" 1.0 (Math|Random|RandomFloatinRange 0.8 1.1) 0.0 "/Game/_Main/Models/RoughModels/DeerMan/Animations/Wendigo_WalkingAttenuation.Wendigo_WalkingAttenuation" 0 0 0))))

(fn ConstructionScript
  (|CallParentFunction))

(fn GetNewTravelLocation
  (bind _randomlocation (Class|NavigationSystemV1|GetRandomLocationinNavigableRadius (Transformation|GetActorLocation) (Variables|Default|GetTravelRadius) 0 0))
  (bind _output_get (Variables|Default|SetCurrentTravelLocation _randomlocation))
  (return _output_get))

(fn SetMovementSpeed
  (params (Movement%20Type :type Enum_EnemyMovementType%20Enum :default "NewEnumerator0"))
  (bind _output_get (Variables|/Script/Engine.CharacterMovementComponent|SetMaxWalkSpeed (Variables|Character|GetCharacterMovement) (Utilities|Select :Index Movement%20Type :NewEnumerator0 0.0 :NewEnumerator1 6e+02 :NewEnumerator2 1.2e+03)))
  (return _output_get))