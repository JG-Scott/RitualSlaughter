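; BP_WeaponMaster is a base hitscan weapon, with empty Recoil and HandleAnimation events as hooks.
; TriggerFire checks ammo and a Tick-driven fire-rate cooldown, calling the player's ThrowWeaponEvent when empty.
; Each shot multi-line traces along camera forward, applies point damage to every hit and optionally makes noise at the player.
; Hits on "Enemy"-tagged actors spawn blood, while other valid hits get stone impacts and temporary bullet-hole decals.
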(event Custom|TriggerFire
  (params (Release :type Boolean) (PlayerRef :type Actor%20Object%20Reference) (CameraLocation :type Vector) (CameraRotation :type Rotator))
  (bind _returnvalue (Game|GetPlayerCharacter 0))
  (if (> (Variables|WeaponStats|GetCurrentAmmo) 0)
    (if (Variables|Default|GetCanFire?)
      (Variables|Default|SetDidFire? true)
      (Variables|PlayerVariables|SetPlayer%20Ref PlayerRef)
      (Variables|PlayerVariables|SetCamera%20Location CameraLocation)
      (Variables|PlayerVariables|SetCamera%20Rotation CameraRotation)
      (CallFunction|HandleAnimation)
      (bind (_location _direction _ignorableactors) (CallFunction|CalculateRayCastDirection (Variables|PlayerVariables|GetCamera%20Location) (Variables|PlayerVariables|GetCamera%20Rotation) (Utilities|Array|MakeArray (Variables|PlayerVariables|GetPlayer%20Ref))))
      (bind _output_get (Variables|Default|SetRayCastDirection _direction))
      (CallFunction|GenerateRayCast (Variables|PlayerVariables|GetCamera%20Location) _output_get _ignorableactors)
      (CallFunction|DealDamage (Variables|Default|GetHitResult))
      (Variables|Default|SetCanFire? false)
      (Utilities|Array|Clear (Variables|Default|GetHitResult))
      (Math|Integer|DecrementInt (Variables|WeaponStats|GetCurrentAmmo)
        (:%20%20
          (if (Variables|Default|GetMakesSound?)
            (Class|Actor|MakeNoise 1.0 _returnvalue (Transformation|GetActorLocation _returnvalue) 0.0 "None"))))
      (else
        (Variables|Default|SetDidFire? false)))
    (else
      (bind _asbp_first_person_character (Utilities|Casting|CastToBP_FirstPersonCharacter PlayerRef))
      (Default|ThrowWeaponEvent _asbp_first_person_character))))

(event Custom|Recoil
  (params (PlayerController :type BP%20First%20Person%20Character%20Object%20Reference)))

(event Custom|HandleAnimation)

(event Custom|GenerateRayCast
  (params (Location :type Vector) (Direction :type Vector) (IgnoreableObjects :type Array%20of%20Actor%20Object%20References))
  ;[1 1 1] Generic create raycast.
  (bind _outhits (Collision|MultiLineTraceByChannel Location Direction "TraceTypeQuery2" true IgnoreableObjects "None"))
  (Variables|Default|SetHitResult _outhits))

(event Custom|DealDamage
  (params (HitResult :type Array%20of%20Hit%20Result%20Structures))
  (bind _player_ref (Variables|PlayerVariables|GetPlayer%20Ref))
  ;[1 1 1] Generic Apply damage
  (bind _array_element (Utilities|Array|ForEachLoopwithBreak HitResult)
    (:LoopBody
      (Game|Damage|ApplyPointDamage (.HitActor (Collision|BreakHitResult _array_element)) (Variables|WeaponStats|GetDamage) (Variables|PlayerVariables|GetCamera%20Location) _array_element (Game|GetInstigatorController _player_ref) _player_ref "/Script/Engine.DamageType")
      ;[1 1 1] Spawn emmitter if shot hits meat
      (Utilities|IsValid (.HitActor (Collision|BreakHitResult _array_element))
        (:Is%20Valid
          (if (Actor|ActorHasTag (.HitActor (Collision|BreakHitResult _array_element)) "Enemy")
            (Effects|SpawnEmitteratLocation "/Game/Realistic_Starter_VFX_Pack_Vol2/Particles/Blood/P_Blood_Splat_Cone.P_Blood_Splat_Cone" (.Location (Collision|BreakHitResult _array_element)) (Math|Conversions|RotationFromXVector (.ImpactNormal (Collision|BreakHitResult _array_element))))
            (else
              (Effects|SpawnEmitteratLocation "/Game/MilitaryWeapDark/FX/P_Impact_Stone_Large_01.P_Impact_Stone_Large_01" (.Location (Collision|BreakHitResult _array_element)) (Math|Conversions|RotationFromXVector (.ImpactNormal (Collision|BreakHitResult _array_element))) "2.000000,2.000000,2.000000")
              (Class|GameplayStatics|SpawnDecalAttached "/Game/_Main/Materials/BulletHoles/BulletHoleDecal.BulletHoleDecal" "15.000000,15.000000,15.000000" (.HitComponent (Collision|BreakHitResult _array_element)) "None" (.Location (Collision|BreakHitResult _array_element)) (Math|Conversions|RotationFromXVector (.ImpactNormal (Collision|BreakHitResult _array_element))) "KeepWorldPosition" 1e+01))))))))

(event Custom|PlayEquipSound
  (Audio|PlaySound2D "/Game/_Main/Sounds/WeaponSoundEffects/ItemEquip.ItemEquip" 1.0 1.0 0.0 0 0))

(event EventBeginPlay)

(event Collision|EventActorBeginOverlap
  (params (OtherActor :type Actor%20Object%20Reference)))

(event EventTick
  (params (DeltaSeconds :type Float%20%28single-precision%29))
  (if (not (Variables|Default|GetCanFire?))
    (bind _output_get (Variables|Default|SetFirerateCounter (+ DeltaSeconds (Variables|Default|GetFirerateCounter))))
    (if (> _output_get (Variables|WeaponStats|GetFireRate))
      (Variables|Default|SetFirerateCounter 0.0)
      (Variables|Default|SetCanFire? true))))

(fn ConstructionScript)

(fn SetRecoilVariables
  (bind _weaponmodel (Variables|Default|GetWeaponModel))
  (bind _weaponmodel_2 (Variables|Default|GetWeaponModel))
  (bind _relativerotation (Variables|/Script/Engine.SceneComponent|GetRelativeRotation _weaponmodel_2))
  (bind _relativelocation (Variables|/Script/Engine.SceneComponent|GetRelativeLocation _weaponmodel))
  (Variables|WeaponStats|SetSetPreRecoilAmount (.pitch _relativerotation))
  (Variables|WeaponStats|SetRecoilRotAmount (+ (.pitch _relativerotation) (Variables|WeaponStats|GetRecoilAmount)))
  (Variables|WeaponStats|SetPreRecoilLocation (.x _relativelocation))
  (Variables|WeaponStats|SetRecoilLocationAmount (+ (.x _relativelocation) (* (Variables|WeaponStats|GetPull%20Back%20Amount) -1.0))))

(fn CalculateRayCastDirection
  (params (CameraLocation :type Vector) (CameraRotation :type Rotator) (Player :type Array%20of%20Actor%20Object%20References))
  (return CameraLocation (+ CameraLocation (* (Math|Vector|GetForwardVector CameraRotation) 1e+05)) Player))

(fn GetYAxis
  (if (< (.Z (Math|Vector|BreakVector (Variables|WeaponStats|GetGunRotation))) 0.0)
    (return false)
    (else
      (return true))))