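; BP_TestRoom is a map-generation room cell whose mesh and cell type are assigned through SetStaticMesh, which also hides its placeholder plane.
; ToggleLight sets the point light's intensity and registers it in the first-person game mode's Lights list.
; GenerateLootBox spawns a supply box at the room's location unless it has an altar.
; GenerateAltar and AddAltar are empty, with their altar-spawning logic left disconnected.
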(event Custom|SetStaticMesh
  (params (New%20Mesh :type Static%20Mesh%20Object%20Reference) (CellType :type Enum_CellType%20Enum :default "NewEnumerator0"))
  (Components|StaticMesh|SetStaticMesh (Variables|Default|GetStaticMesh) New%20Mesh)
  (Variables|Default|SetCellType CellType)
  (Rendering|SetVisibility (Variables|Default|GetPlane) false false))

(event Custom|ToggleLight
  (Rendering|Components|Light|SetIntensity (Variables|Default|GetPointLight) 5e+03)
  (bind _asbp_first_person_game_mode (Utilities|Casting|CastToBP_FirstPersonGameMode (Game|GetGameMode)))
  (Utilities|Array|Add (Variables|/Game/FirstPerson/Blueprints/BP_FirstPersonGameMode.BP_FirstPersonGameMode_C|GetLights _asbp_first_person_game_mode) (Variables|Default|GetPointLight)))

(event Custom|GenerateLootBox
  (if (not (Variables|Default|GetHasAltar))
    (Game|SpawnActorfromClass "/Game/_Main/Props/Interactables/BP_SupplyBoxInteract.BP_SupplyBoxInteract_C" (Math|Transform|MakeTransform (Transformation|GetActorLocation) "0, 0, 0" "1.000000,1.000000,1.000000") "AdjustIfPossibleButAlwaysSpawn" "MultiplyWithRoot" 0 0)
    (Variables|Default|SetHasLootBox true)))

(event Custom|GenerateAltar)

(event EventBeginPlay)

(event Collision|EventActorBeginOverlap
  (params (OtherActor :type Actor%20Object%20Reference)))

(event EventTick
  (params (DeltaSeconds :type Float%20%28single-precision%29)))

(fn ConstructionScript)

(fn Model
  (return (== (Variables|Default|GetStaticMesh) "/Game/_Main/Models/RoughModels/MapGeneration/BaseCube2.BaseCube2")))

(fn AddAltar)