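; Custom point/spot light actor that publishes its settings to the MPC_GlobalLighting material parameter collection, in one of eight slots chosen by clamped LightIndex.
; Constructor writes location, radius, colours, brightness and spot cone parameters under index-suffixed names, taking direction from the Arrow and resizing the PointRadius sphere.
; The construction script and Update event run Constructor.
; DisableLight zeroes the slot's brightness and also runs on BeginPlay, so lights start off.
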(event Custom|Update
  (CallFunction|Constructor))

(event Custom|DisableLight
  (Rendering|Material|SetScalarParameterValue "/Game/GouraudPhong/Materials/MPC_GlobalLighting.MPC_GlobalLighting" (Utilities|String|StringToName (Utilities|String|Append "PointBrightness" (Utilities|String|ToString(Integer) (Math|Integer|Clamp(Integer) (Variables|Default|GetLightIndex) 0 7)))) 0.0 :!class /Script/Engine.KismetMaterialLibrary))

(event EventBeginPlay
  (CallFunction|DisableLight))

(fn ConstructionScript
  (CallFunction|Constructor))

(fn Constructor
  (bind _lightindex (Variables|Default|GetLightIndex))
  (bind _radius (Variables|PointLight|GetRadius))
  (bind _returnvalue (Math|Integer|Clamp(Integer) _lightindex 0 7))
  (bind _returnvalue_2 (Utilities|String|ToString(Integer) _returnvalue))
  ;[1 1 1] Point Light
  (Rendering|Material|SetVectorParameterValue "/Game/GouraudPhong/Materials/MPC_GlobalLighting.MPC_GlobalLighting" (Utilities|String|StringToName (Utilities|String|Append "PointLocation" _returnvalue_2)) (Math|Conversions|ToLinearColor(Vector) (Transformation|GetActorLocation)) :!class /Script/Engine.KismetMaterialLibrary)
  (Components|Sphere|SetSphereRadius (Variables|Default|GetPointRadius) _radius true)
  (Rendering|Material|SetScalarParameterValue "/Game/GouraudPhong/Materials/MPC_GlobalLighting.MPC_GlobalLighting" (Utilities|String|StringToName (Utilities|String|Append "PointRadius" _returnvalue_2)) _radius :!class /Script/Engine.KismetMaterialLibrary)
  (Rendering|Material|SetVectorParameterValue "/Game/GouraudPhong/Materials/MPC_GlobalLighting.MPC_GlobalLighting" (Utilities|String|StringToName (Utilities|String|Append "PointColour" _returnvalue_2)) (Variables|PointLight|GetPointColour) :!class /Script/Engine.KismetMaterialLibrary)
  (Rendering|Material|SetVectorParameterValue "/Game/GouraudPhong/Materials/MPC_GlobalLighting.MPC_GlobalLighting" (Utilities|String|StringToName (Utilities|String|Append "PointSpecular" _returnvalue_2)) (Variables|PointLight|GetPointSpecular) :!class /Script/Engine.KismetMaterialLibrary)
  (Rendering|Material|SetScalarParameterValue "/Game/GouraudPhong/Materials/MPC_GlobalLighting.MPC_GlobalLighting" (Utilities|String|StringToName (Utilities|String|Append "PointBrightness" _returnvalue_2)) (Variables|PointLight|GetPointBrightness) :!class /Script/Engine.KismetMaterialLibrary)
  ;[1 1 1] Spot Light
  (Rendering|Material|SetScalarParameterValue "/Game/GouraudPhong/Materials/MPC_GlobalLighting.MPC_GlobalLighting" (Utilities|String|StringToName (Utilities|String|Append "SpotAngle" _returnvalue_2)) (Variables|SpotLight|GetSpotAngle) :!class /Script/Engine.KismetMaterialLibrary)
  (Rendering|Material|SetVectorParameterValue "/Game/GouraudPhong/Materials/MPC_GlobalLighting.MPC_GlobalLighting" (Utilities|String|StringToName (Utilities|String|Append "SpotDirection" _returnvalue_2)) (Math|Conversions|ToLinearColor(Vector) (Math|Vector|Normalize (Math|Vector|GetForwardVector (Variables|Default|GetArrow)))) :!class /Script/Engine.KismetMaterialLibrary)
  (Rendering|Material|SetScalarParameterValue "/Game/GouraudPhong/Materials/MPC_GlobalLighting.MPC_GlobalLighting" (Utilities|String|StringToName (Utilities|String|Append "SpotSoftness" _returnvalue_2)) (Variables|SpotLight|GetSpotSoftness) :!class /Script/Engine.KismetMaterialLibrary))