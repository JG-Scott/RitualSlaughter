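; Interactable altar that the player destroys by holding interact for about five seconds.
; Interact toggles the hold; Tick then accumulates a timer into the HUD progress bar and plays a break sound via DoOnce.
; Releasing resets progress, while leaving PickupRadius stops the hold without resetting the timer.
; Completion spawns gore effects and BP_BrokenAltar, plays sounds, emits loud noise, notifies BP_FirstPersonGameMode and destroys the actor.
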(event OnComponentEndOverlap(PickupRadius)
  (params (OverlappedComponent :type Primitive%20Component%20Object%20Reference) (OtherActor :type Actor%20Object%20Reference) (OtherComp :type Primitive%20Component%20Object%20Reference) (OtherBodyIndex :type Integer))
  (Utilities|Casting|CastToBP_FirstPersonCharacter OtherActor)
  (if (Variables|Default|GetIsHeldDown)
    (Variables|Default|SetIsHeldDown false)
    (Default|SetProgressBarVisibility (Variables|/Game/FirstPerson/Blueprints/BP_FirstPersonCharacter.BP_FirstPersonCharacter_C|GetMainHUDRef (Variables|Default|GetCharacterInteracting)) false)))

(event Custom|Explode
  (bind _returnvalue (Transformation|GetActorLocation))
  (bind _returnvalue_2 (+ _returnvalue "0.000000,0.000000,200.000000"))
  (for _index (range 0 1)
    (Niagara|SpawnSystematLocation "/Game/_Main/ParticleEffects/ThrowableItemParticles/NS_BloodExplosion1.NS_BloodExplosion1" _returnvalue_2 "0, 0, 0" "5.000000,5.000000,5.000000")
    (Niagara|SpawnSystematLocation "/Game/_Main/ParticleEffects/BloodSplatter/NS_GibletExplosion.NS_GibletExplosion" _returnvalue_2))
  (Game|SpawnActorfromClass "/Game/_Main/Props/Altar/BP_BrokenAltar.BP_BrokenAltar_C" (Math|Transform|MakeTransform _returnvalue "0, 0, 0" "1.000000,1.000000,1.000000") "Undefined" "MultiplyWithRoot" 0 0)
  (Audio|Components|Audio|Stop (Variables|Default|GetBreakSound))
  (CallFunction|PlayDestroySounds)
  (bind _asbp_first_person_game_mode (Utilities|Casting|CastToBP_FirstPersonGameMode (Game|GetGameMode)))
  (Default|AltarDestroyed _asbp_first_person_game_mode)
  (Actor|DestroyActor))

(event Custom|PlayDestroySounds
  (Audio|PlaySound2D "/Game/StarterContent/Audio/Explosion01.Explosion01" 0.5 1.0 0.0 0 0)
  (Audio|PlaySound2D "/Game/_Main/Sounds/AltarSounds/RubbleCue.RubbleCue" 2.0 1.0 0.0 0 0)
  (Audio|PlaySound2D "/Game/_Main/Sounds/AltarSounds/brokenAltarScream.brokenAltarScream" 0.5 1.0 0.0 0 0)
  (Class|Actor|MakeNoise 2e+03 (Game|GetPlayerCharacter 0) "0, 0, 0" 0.0 "None"))

(event EventBeginPlay
  (|CallParentFunction))

(event Collision|EventActorBeginOverlap
  (params (OtherActor :type Actor%20Object%20Reference))
  (|CallParentFunction OtherActor) ; This node is disabled and will not be called.\nDrag off pins to build functionality.
)

(event EventTick
  (params (DeltaSeconds :type Float%20%28single-precision%29))
  (|CallParentFunction DeltaSeconds)
  (if (Variables|Default|GetIsHeldDown)
    (Utilities|FlowControl|Sequence
      (:then_0
        (Utilities|FlowControl|DoOnce false :!label _label
          (:Completed
            (bind _returnvalue (Audio|SpawnSound2D "/Game/_Main/Sounds/AltarSounds/dummyNextToYaNoise_1.dummyNextToYaNoise_1" 1.0 1.0 0.0 0))
            (Variables|Default|SetBreakSound _returnvalue))))
      (:then_1
        (bind _output_get (Variables|Default|SetTimer (+ (Variables|Default|GetTimer) DeltaSeconds)))
        (bind _output_get_2 (Variables|/Game/_Main/Widgets/PlayerUI/MainHUD.MainHUD_C|SetInteractProgressBarValue (Variables|/Game/FirstPerson/Blueprints/BP_FirstPersonCharacter.BP_FirstPersonCharacter_C|GetMainHUDRef (Variables|Default|GetCharacterInteracting)) _output_get))
        (if (>= _output_get_2 5.0)
          (CallFunction|Explode))))
    (else
      (Utilities|IsValid (Variables|Default|GetBreakSound)
        (:Is%20Valid
          (Audio|Components|Audio|Stop (Variables|Default|GetBreakSound))
          (goto _label Reset))))))

(event EventInteract
  (params (CharacterPickingUp :type BP%20First%20Person%20Character%20Object%20Reference) (ActionValue :type Boolean))
  (Development|PrintString "Hello")
  (bind _output_get (Variables|Default|SetCharacterInteracting CharacterPickingUp))
  (bind _output_get_2 (Variables|Default|SetIsHeldDown ActionValue))
  (if _output_get_2
    (Default|SetProgressBarVisibility (Variables|/Game/FirstPerson/Blueprints/BP_FirstPersonCharacter.BP_FirstPersonCharacter_C|GetMainHUDRef _output_get) true)
    (elif (> (Variables|Default|GetTimer) 0.0)
      (bind _output_get_3 (Variables|Default|SetTimer (Variables|Default|GetTimerStartingValue)))
      (Variables|/Game/_Main/Widgets/PlayerUI/MainHUD.MainHUD_C|SetInteractProgressBarValue (Variables|/Game/FirstPerson/Blueprints/BP_FirstPersonCharacter.BP_FirstPersonCharacter_C|GetMainHUDRef (Variables|Default|GetCharacterInteracting)) _output_get_3)
      (Default|SetProgressBarVisibility (Variables|/Game/FirstPerson/Blueprints/BP_FirstPersonCharacter.BP_FirstPersonCharacter_C|GetMainHUDRef (Variables|Default|GetCharacterInteracting)) false))))

(fn ConstructionScript
  (|CallParentFunction))